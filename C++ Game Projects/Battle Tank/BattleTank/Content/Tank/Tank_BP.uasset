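; Player-controllable tank Blueprint that wires up its aiming, track movement and health bar on BeginPlay.
; The aiming component receives the barrel and turret, and the movement component receives both tracks.
; Input axes rotate a gimbal and spring arm for a frame-rate-independent orbit camera, or pass move and turn intents to the movement component.
; Fire input calls the aiming component, and the health bar widget stores a reference to this tank.
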(event EventBeginPlay
  (Class|TankAimingComponet|Initialise (Variables|Default|GetTankAimingComponet) (Variables|Default|GetTankBarrel) (Variables|Default|GetTankTurret))
  (Class|TankMovementComponent|Initialise (Variables|Default|GetTankMovement) (Variables|Default|GetLeftTrack) (Variables|Default|GetRightTrack))
  (CallFunction|InitialiseHealthBarWidget))

(event Input|ActionEvents|InputActionFire
  (params (Key :type Key%20Structure))
  ;[1 1 1] Firing Input
  (:Pressed
    (Class|TankAimingComponet|Fire (Variables|Default|GetTankAimingComponet))))

(event Input|AxisEvents|InputAxisAimAzimuth
  (params (AxisValue :type Float%20%28single-precision%29))
  ;[1 1 1] Camera
  (Transformation|AddLocalRotation (Variables|Default|GetAzimuthGimbol) (Math|Rotator|MakeRotator 0.0 0.0 (* AxisValue (Utilities|Time|GetWorldDeltaSeconds) 1e+02)) false false))

(event Input|AxisEvents|InputAxisAimElevation
  (params (AxisValue :type Float%20%28single-precision%29))
  ;[1 1 1] Camera
  (Transformation|AddLocalRotation (Variables|Default|GetSpringArm) (Math|Rotator|MakeRotator 0.0 (* AxisValue (Utilities|Time|GetWorldDeltaSeconds) 1e+02) 0.0) false false))

(event Input|AxisEvents|InputAxisTurnRight
  (params (AxisValue :type Float%20%28single-precision%29))
  ;[1 1 1] Movement Binding
  (Class|TankMovementComponent|IntendTurnRight (Variables|Default|GetTankMovement) AxisValue))

(event Input|AxisEvents|InputAxisMoveForward
  (params (AxisValue :type Float%20%28single-precision%29))
  ;[1 1 1] Movement Binding
  (Class|TankMovementComponent|IntendMoveForward (Variables|Default|GetTankMovement) AxisValue))

(fn ConstructionScript)

(fn InitialiseHealthBarWidget
  (bind _ashealth_bar (Utilities|Casting|CastToHealthBar (UserInterface|GetUserWidgetObject (Variables|Default|GetWidget))))
  (Variables|/Game/Blueprints/HealthBar.HealthBar_C|SetTank.%20Reference _ashealth_bar self))